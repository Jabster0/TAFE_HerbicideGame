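; Melee enemy character that chases the player, attacks and drops loot on death.
; Pawn sensing latches IsSeeingPlayer and starts an AI move to the player; until then, Tick halts movement.
; On arrival it plays a punch montage and damages the player immediately, gated by CanAttack.
; At zero health it may drop random health, shield or ammo pickups at nearby reachable points, then destroys itself.
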(event OnSeePawn(PawnSensing)
  (params (Pawn :type Pawn%20Object%20Reference))
  ;[1 1 1] Enemy AI
  (Variables|Default|SetisSeeingPlayer? true)
  (CallFunction|FollowPlayer))

(event Custom|DropLoot
  (bind _returnvalue (Transformation|GetActorLocation))
  (bind _outhit (Collision|LineTraceByChannel _returnvalue (- _returnvalue "0.000000,0.000000,200.000000") "TraceTypeQuery1" false (Utilities|Array|MakeArray (Game|GetPlayerCharacter 0)) "None"))
  (Game|SpawnActorfromClass (Utilities|Select :Index (Math|Random|RandomInteger 5) :Option%200 "/Game/Blueprints/BP_50Healthpick.BP_50Healthpick_C" :Option%201 "/Game/Blueprints/BP_50Shieldpick1.BP_50Shieldpick1_C" :Option%202 "/Game/Blueprints/BP_AmmoPickup.BP_AmmoPickup_C" :Option%203 "/Game/Blueprints/BP_50Shieldpick1.BP_50Shieldpick1_C" :Option%204 "/Game/Blueprints/BP_50Shieldpick1.BP_50Shieldpick1_C" :Option%205 "/Game/Blueprints/BP_AmmoPickup.BP_AmmoPickup_C" :Option%206 "/Game/Blueprints/BP_AmmoPickup.BP_AmmoPickup_C") (Math|Transform|MakeTransform (.RandomLocation (AI|Navigation|GetRandomReachablePointinRadius (.Location (Collision|BreakHitResult _outhit)) 2.5e+02 0 0)) (Math|Rotator|MakeRotator 0.0 0.0 (Math|Random|RandomFloatinRange 0.0 3.6e+02))) "Undefined" "MultiplyWithRoot" 0 0))

(event Custom|FollowPlayer
  ;[1 1 1] Enemy AI
  (Variables|Default|SetcanAttack? true)
  (if (Variables|Default|GetisSeeingPlayer?)
    (AI|AIMoveTo self "0, 0, 0" (Game|GetPlayerCharacter 0) 7e+01 false
      (:OnSuccess
        (if (Variables|Default|GetcanAttack?)
          (Variables|Default|SetcanAttack? false)
          (bind _returnvalue (Animation|PlayAnimMontage "/Game/Animations/Animation/Paired_CounterPunch_PalmStrike_Att_Montage.Paired_CounterPunch_PalmStrike_Att_Montage" 1.0 "None"))
          (CallFunction|DoingDamage)
          (Utilities|FlowControl|Delay _returnvalue)
          (Variables|Default|SetcanAttack? true))))
    (else
      (Variables|Default|SetisSeeingPlayer? false))))

(event Custom|DoingDamage
  ;[1 1 1] Damage
  (bind _asbp_first_person_character (Utilities|Casting|CastToBP_FirstPersonCharacter (Game|GetPlayerCharacter 0)))
  (Game|Damage|ApplyDamage _asbp_first_person_character 0.1 0 self))

(event EventBeginPlay)

(event Collision|EventActorBeginOverlap
  (params (OtherActor :type Actor%20Object%20Reference)))

(event EventTick
  (params (DeltaSeconds :type Float%20%28single-precision%29))
  ;[1 1 1] Enemy AI
  (if (not (Variables|Default|GetisSeeingPlayer?))
    (Components|Movement|StopMovementImmediately (Variables|Character|GetCharacterMovement))))

(event Game|Damage|EventAnyDamage
  (params (Damage :type Float%20%28single-precision%29) (DamageType :type Damage%20Type%20Object%20Reference) (InstigatedBy :type Controller%20Object%20Reference) (DamageCauser :type Actor%20Object%20Reference))
  ;[1 1 1] Health System
  (Variables|Default|SetHealth (- (Variables|Default|GetHealth) Damage))
  (if (<= (Variables|Default|GetHealth) 0.0)
    (for _index (range 0 (Math|Random|RandomInteger 2))
      (CallFunction|DropLoot))
    (Actor|DestroyActor)))

(fn ConstructionScript)