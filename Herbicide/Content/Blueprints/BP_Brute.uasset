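; Brute melee enemy that chases the player on PawnSensing sight, attacks, and drops random pickups on death.
; AIMoveTo success starts a montage combo indexed by AttackIndex, with SaveAttack intended to chain up to four swings.
; Hand collisions attached to mesh sockets deal damage and camera shake on overlap; the sphere-trace alternative is unwired.
; At zero health it disables collision and movement, plays a death montage, ragdolls, then destroys itself.
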(event OnSeePawn(PawnSensing)
  (params (Pawn :type Pawn%20Object%20Reference))
  ;[1 1 1] Enemy AI
  (Variables|Default|SetisSeeingPlayer? true)
  (CallFunction|FollowPlayer))

(event OnComponentBeginOverlap(RightHandCollision)
  (params (OverlappedComponent :type Primitive%20Component%20Object%20Reference) (OtherActor :type Actor%20Object%20Reference) (OtherComp :type Primitive%20Component%20Object%20Reference) (OtherBodyIndex :type Integer) (bFromSweep :type Boolean) (SweepResult :type Hit%20Result%20Structure%20%28by%20ref%29))
  ;[1 1 1] Damage
  (bind _asbp_first_person_character (Utilities|Casting|CastToBP_FirstPersonCharacter OtherActor))
  (Game|Damage|ApplyDamage _asbp_first_person_character 0.2 0 self)
  (Camera|PlayWorldCameraShake "/Script/Engine.CameraShakeBase" "0, 0, 0" 0.0 0.0))

(event OnComponentBeginOverlap(LeftHandCollision)
  (params (OverlappedComponent :type Primitive%20Component%20Object%20Reference) (OtherActor :type Actor%20Object%20Reference) (OtherComp :type Primitive%20Component%20Object%20Reference) (OtherBodyIndex :type Integer) (bFromSweep :type Boolean) (SweepResult :type Hit%20Result%20Structure%20%28by%20ref%29))
  ;[1 1 1] Damage
  (bind _asbp_first_person_character (Utilities|Casting|CastToBP_FirstPersonCharacter OtherActor))
  (Game|Damage|ApplyDamage _asbp_first_person_character 0.2 0 self)
  (Camera|PlayWorldCameraShake "/Script/Engine.CameraShakeBase" "0, 0, 0" 0.0 0.0))

(event Custom|DropLoot
  (bind _returnvalue (Transformation|GetActorLocation))
  ;[1 1 1] Loot drops
  (bind _outhit (Collision|LineTraceByChannel _returnvalue (- _returnvalue "0.000000,0.000000,200.000000") "TraceTypeQuery1" false (Utilities|Array|MakeArray (Game|GetPlayerCharacter 0)) "None"))
  (Game|SpawnActorfromClass (Utilities|Select :Index (Math|Random|RandomInteger 5) :Option%200 "/Game/Blueprints/BP_50Healthpick.BP_50Healthpick_C" :Option%201 "/Game/Blueprints/BP_50Shieldpick1.BP_50Shieldpick1_C" :Option%202 "/Game/Blueprints/BP_AmmoPickup.BP_AmmoPickup_C" :Option%203 "/Game/Blueprints/BP_50Shieldpick1.BP_50Shieldpick1_C" :Option%204 "/Game/Blueprints/BP_50Shieldpick1.BP_50Shieldpick1_C" :Option%205 "/Game/Blueprints/BP_AmmoPickup.BP_AmmoPickup_C" :Option%206 "/Game/Blueprints/BP_AmmoPickup.BP_AmmoPickup_C") (Math|Transform|MakeTransform (.RandomLocation (AI|Navigation|GetRandomReachablePointinRadius (.Location (Collision|BreakHitResult _outhit)) 2.5e+02 0 0)) (Math|Rotator|MakeRotator 0.0 0.0 (Math|Random|RandomFloatinRange 0.0 3.6e+02))) "Undefined" "MultiplyWithRoot" 0 0))

(event Custom|FollowPlayer
  ;[1 1 1] Enemy AI
  (Variables|Default|SetcanAttack? true)
  (if (Variables|Default|GetisSeeingPlayer?)
    (AI|AIMoveTo self "0, 0, 0" (Game|GetPlayerCharacter 0) 1e+02 false
      (:OnSuccess
        (if (Variables|Default|GetcanAttack?)
          (CallFunction|BruteMelee))))
    (else
      (Variables|Default|SetisSeeingPlayer? false))))

(event Custom|Attack_reset
  ;[1 1 1] Enemy AI
  (Utilities|FlowControl|DoOnce false) ; enters at Reset
)

(event Custom|StopMeleeCombo
  ;[1 1 1] StopMelee
  (Variables|Default|SetIsAttacking? false)
  (Variables|Default|SetAttackIndex 0))

(event Custom|LhandTrace
  ;[1 0 0] Sphere trace melee system. (Doesnt work...yet)
)

(event Custom|RhandTrace
  ;[1 0 0] Sphere trace melee system. (Doesnt work...yet)
)

(event Custom|StartLhandTrace
  ;[1 0 0] Sphere trace melee system. (Doesnt work...yet)
)

(event Custom|BruteMeleeCombo
  ;[1 1 1] ComboContinues
  (if (Variables|Default|GetsaveAttack?)
    (Variables|Default|SetsaveAttack? false)
    (switch int (Variables|Default|GetAttackIndex)
      (:0
        (CallFunction|Attack1))
      (:1
        (CallFunction|Attack2))
      (:2
        (CallFunction|Attack3))
      (:3
        (CallFunction|Attack4)))
    (else
      (CallFunction|StopMeleeCombo)
      (CallFunction|FollowPlayer))))

(event Custom|StartRhandTimer
  ;[1 0 0] Sphere trace melee system. (Doesnt work...yet)
)

(event Custom|StopTraceTimer
  ;[1 0 0] Sphere trace melee system. (Doesnt work...yet)
  (Utilities|Time|ClearandInvalidateTimerbyHandle (Variables|Default|GetRhandTimer)))

(event Custom|Attack%204
  ;[0.03646 0.03646 0.03646] Attack 4
  (Utilities|FlowControl|DoOnce false :!label _label
    (:Completed
      (Utilities|FlowControl|Delay 0.1)
      (Animation|Montage|PlayMontage (Variables|Character|GetMesh) "/Game/Characters/Enemies/Brute/Animations/AM_BruteSwipingR.AM_BruteSwipingR"
        (:then
          (Variables|Default|SetAttackIndex 4)
          (goto _label Reset))))))

(event Custom|Attack%201
  ;[0.03646 0.03646 0.03646] Attack 1
  (Utilities|FlowControl|DoOnce false :!label _label
    (:Completed
      (Utilities|FlowControl|Delay 0.1)
      (Animation|Montage|PlayMontage (Variables|Character|GetMesh) "/Game/Characters/Enemies/Brute/Animations/AM_BruteSwipingL.AM_BruteSwipingL"
        (:then
          (Variables|Default|SetAttackIndex 1)
          (goto _label Reset))))))

(event Custom|Attack%202
  ;[0.03646 0.03646 0.03646] Attack 2
  (Utilities|FlowControl|DoOnce false :!label _label
    (:Completed
      (Utilities|FlowControl|Delay 0.1)
      (Animation|Montage|PlayMontage (Variables|Character|GetMesh) "/Game/Characters/Enemies/Brute/Animations/AM_BrutePunchR2.AM_BrutePunchR2"
        (:then
          (Variables|Default|SetAttackIndex 2)
          (goto _label Reset))))))

(event Custom|Attack%203
  ;[0.03646 0.03646 0.03646] Attack 3
  (Utilities|FlowControl|DoOnce false :!label _label
    (:Completed
      (Utilities|FlowControl|Delay 0.1)
      (Animation|Montage|PlayMontage (Variables|Character|GetMesh) "/Game/Characters/Enemies/Brute/Animations/AM_BrutePunchL2.AM_BrutePunchL2"
        (:then
          (Variables|Default|SetAttackIndex 3)
          (goto _label Reset))))))

(event Custom|BruteMelee
  ;[1 1 1] Melee attack
  (if (Variables|Default|GetIsAttacking?)
    (Variables|Default|SetsaveAttack? true)
    (else
      (Variables|Default|SetIsAttacking? true)
      (switch int (Variables|Default|GetAttackIndex)
        (:0
          (CallFunction|Attack1))
        (:1
          (CallFunction|Attack2))
        (:2
          (CallFunction|Attack3))
        (:3
          (CallFunction|Attack4))))))

(event Collision|EventActorBeginOverlap
  (params (OtherActor :type Actor%20Object%20Reference)))

(event EventTick
  (params (DeltaSeconds :type Float%20%28single-precision%29))
  ;[1 1 1] Enemy AI
  (if (not (Variables|Default|GetisSeeingPlayer?))
    (Components|Movement|StopMovementImmediately (Variables|Character|GetCharacterMovement))))

(event Game|Damage|EventAnyDamage
  (params (Damage :type Float%20%28single-precision%29) (DamageType :type Damage%20Type%20Object%20Reference) (InstigatedBy :type Controller%20Object%20Reference) (DamageCauser :type Actor%20Object%20Reference))
  ;[1 1 1] Health System
  (Variables|Default|SetHealth (- (Variables|Default|GetHealth) Damage))
  (if (<= (Variables|Default|GetHealth) 0.0)
    (for _index (range 0 (Math|Random|RandomInteger 2))
      (CallFunction|DropLoot))
    (Collision|SetCollisionEnabled (Variables|Collision|GetCapsuleComponent) "NoCollision")
    (Collision|SetCollisionEnabled (Variables|Character|GetMesh) "PhysicsOnly")
    (Pawn|Components|CharacterMovement|DisableMovement (Variables|Character|GetCharacterMovement))
    (Animation|PlayAnimMontage "/Game/Characters/Enemies/Brute/Animations/AM_BruteDeath.AM_BruteDeath" 1.0 "None")
    (Utilities|FlowControl|Delay 3.6)
    (Physics|SetSimulatePhysics (Variables|Character|GetMesh) true)
    (Utilities|FlowControl|Delay 1e+01)
    (Actor|DestroyActor)))

(fn ConstructionScript
  (bind _mesh (Variables|Character|GetMesh))
  (Transformation|AttachComponentToComponent (Variables|Default|GetLeftHandCollision) _mesh "LeftHand" "KeepRelative" "KeepRelative" "KeepRelative" true)
  (Transformation|AttachComponentToComponent (Variables|Default|GetRightHandCollision) _mesh "RightHand" "KeepRelative" "KeepRelative" "KeepRelative" true))