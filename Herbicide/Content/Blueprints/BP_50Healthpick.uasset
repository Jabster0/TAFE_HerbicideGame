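; BP_50Healthpick is a health pickup that restores half of the player's normalized health.
; Overlapping its collision component casts to BP_FirstPersonCharacter, adds to Health capped at full, prints the new value as debug text and destroys the pickup.
; An uncollected pickup destroys itself after a fixed delay from BeginPlay.
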(event OnComponentBeginOverlap(Collisonspear)
  (params (OverlappedComponent :type Primitive%20Component%20Object%20Reference) (OtherActor :type Actor%20Object%20Reference) (OtherComp :type Primitive%20Component%20Object%20Reference) (OtherBodyIndex :type Integer) (bFromSweep :type Boolean) (SweepResult :type Hit%20Result%20Structure%20%28by%20ref%29))
  (bind _asbp_first_person_character (Utilities|Casting|CastToBP_FirstPersonCharacter OtherActor))
  (bind _output_get (Variables|Default|SetAs%20BP%20First%20Person%20Character _asbp_first_person_character))
  (Variables|/Game/FirstPerson/Blueprints/BP_FirstPersonCharacter.BP_FirstPersonCharacter_C|SetHealth _output_get (+ (Variables|/Game/FirstPerson/Blueprints/BP_FirstPersonCharacter.BP_FirstPersonCharacter_C|GetHealth (Variables|Default|GetAs%20BP%20First%20Person%20Character)) 0.5))
  (if (>= (Variables|/Game/FirstPerson/Blueprints/BP_FirstPersonCharacter.BP_FirstPersonCharacter_C|GetHealth (Variables|Default|GetAs%20BP%20First%20Person%20Character)) 1.0)
    (Variables|/Game/FirstPerson/Blueprints/BP_FirstPersonCharacter.BP_FirstPersonCharacter_C|SetHealth (Variables|Default|GetAs%20BP%20First%20Person%20Character) 1.0))
  (Development|PrintString "Health")
  (Development|PrintString (Utilities|String|ToString(Float) (Variables|/Game/FirstPerson/Blueprints/BP_FirstPersonCharacter.BP_FirstPersonCharacter_C|GetHealth (Variables|Default|GetAs%20BP%20First%20Person%20Character))))
  (Actor|DestroyActor))

(event EventBeginPlay
  (Utilities|FlowControl|Delay 2e+01)
  (Actor|DestroyActor))

(fn ConstructionScript)