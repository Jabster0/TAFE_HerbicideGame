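; BP_AmmoPickup is a pickup that refills the first-person character's pistol reserve ammo.
; On BeginPlay it caches the first BP_FirstPersonCharacter found in the level.
; When that character class overlaps Sphere1, it adds a fixed amount to the cached character's PistolTotalAmmo, capped at a maximum.
; It then prints the new total and destroys itself.
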(event OnComponentBeginOverlap(Sphere1)
  (params (OverlappedComponent :type Primitive%20Component%20Object%20Reference) (OtherActor :type Actor%20Object%20Reference) (OtherComp :type Primitive%20Component%20Object%20Reference) (OtherBodyIndex :type Integer) (bFromSweep :type Boolean) (SweepResult :type Hit%20Result%20Structure%20%28by%20ref%29))
  (Utilities|Casting|CastToBP_FirstPersonCharacter OtherActor)
  (Variables|/Game/FirstPerson/BluePrints/BP_FirstPersonCharacter.BP_FirstPersonCharacter_C|SetPistolTotalAmmo (Variables|Default|GetFirst%20Person%20Character) (+ (Variables|/Game/FirstPerson/BluePrints/BP_FirstPersonCharacter.BP_FirstPersonCharacter_C|GetPistolTotalAmmo (Variables|Default|GetFirst%20Person%20Character)) 2e+01))
  (if (>= (Variables|/Game/FirstPerson/BluePrints/BP_FirstPersonCharacter.BP_FirstPersonCharacter_C|GetPistolTotalAmmo (Variables|Default|GetFirst%20Person%20Character)) 1e+02)
    (Variables|/Game/FirstPerson/BluePrints/BP_FirstPersonCharacter.BP_FirstPersonCharacter_C|SetPistolTotalAmmo (Variables|Default|GetFirst%20Person%20Character) 1e+02))
  (Development|PrintString "Total Ammo")
  (Development|PrintString (Utilities|String|ToString(Float) (Variables|/Game/FirstPerson/BluePrints/BP_FirstPersonCharacter.BP_FirstPersonCharacter_C|GetPistolTotalAmmo (Variables|Default|GetFirst%20Person%20Character))))
  (Actor|DestroyActor))

(event EventBeginPlay
  (bind _outactors (Actor|GetAllActorsOfClass "/Game/FirstPerson/BluePrints/BP_FirstPersonCharacter.BP_FirstPersonCharacter_C"))
  (Variables|Default|SetFirst%20Person%20Character (Utilities|Array|Get(acopy) _outactors)))

(fn ConstructionScript)