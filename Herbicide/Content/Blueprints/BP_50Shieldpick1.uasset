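; BP_50Shieldpick1 is a shield pickup that grants the first-person character 50 shield points.
; An overlap on its collision component casts the other actor to BP_FirstPersonCharacter and ignores anything else.
; It adds to the character's Shield, caps it at 100, prints the new value for debugging and destroys itself.
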(event OnComponentBeginOverlap(Collisonspear)
  (params (OverlappedComponent :type Primitive%20Component%20Object%20Reference) (OtherActor :type Actor%20Object%20Reference) (OtherComp :type Primitive%20Component%20Object%20Reference) (OtherBodyIndex :type Integer) (bFromSweep :type Boolean) (SweepResult :type Hit%20Result%20Structure%20%28by%20ref%29))
  (bind _asbp_first_person_character (Utilities|Casting|CastToBP_FirstPersonCharacter OtherActor))
  (bind _output_get (Variables|Default|SetAs%20BP%20First%20Person%20Character _asbp_first_person_character))
  (Variables|/Game/FirstPerson/BluePrints/BP_FirstPersonCharacter.BP_FirstPersonCharacter_C|SetShield _output_get (+ (Variables|/Game/FirstPerson/BluePrints/BP_FirstPersonCharacter.BP_FirstPersonCharacter_C|GetShield (Variables|Default|GetAs%20BP%20First%20Person%20Character)) 5e+01))
  (if (>= (Variables|/Game/FirstPerson/BluePrints/BP_FirstPersonCharacter.BP_FirstPersonCharacter_C|GetShield (Variables|Default|GetAs%20BP%20First%20Person%20Character)) 1e+02)
    (Variables|/Game/FirstPerson/BluePrints/BP_FirstPersonCharacter.BP_FirstPersonCharacter_C|SetShield (Variables|Default|GetAs%20BP%20First%20Person%20Character) 1e+02))
  (Development|PrintString "Shield")
  (Development|PrintString (Utilities|String|ToString(Float) (Variables|/Game/FirstPerson/BluePrints/BP_FirstPersonCharacter.BP_FirstPersonCharacter_C|GetShield (Variables|Default|GetAs%20BP%20First%20Person%20Character))))
  (Actor|DestroyActor))

(fn ConstructionScript)